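; Tic-tac-toe style 3x3 grid actor that fills cells on overlap and checks for three in a row.
; Each box's first overlap adds a static mesh, writes its GrilleArray entry, calls TestingWin, then changes collision after a short delay; boxes 8 and 9 set BoxEnable7.
; TestingWin checks the played row, the first cell's column and both diagonals, printing "Win" on a match.
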(event OnComponentBeginOverlap(Box_1)
  (params (OverlappedComponent :type Primitive%20Component%20Object%20Reference) (OtherActor :type Actor%20Object%20Reference) (OtherComp :type Primitive%20Component%20Object%20Reference) (OtherBodyIndex :type Integer) (bFromSweep :type Boolean) (SweepResult :type Hit%20Result%20Structure%20%28by%20ref%29))
  (bind _box_1 (Variables|Default|GetBox_1))
  (bind _returnvalue (Transformation|GetRelativeTransform _box_1))
  (if (not (Variables|Default|GetBoxEnable1))
    (AddComponent|AddStaticMeshComponent false (Math|Transform|MakeTransform (.location _returnvalue) (.rotation _returnvalue) "1.000000,1.000000,1.000000"))
    (Variables|Default|SetBoxEnable1 true)
    (Utilities|Array|SetArrayElem (Variables|Default|GetGrilleArray) 0 (Utilities|Struct|MakeStruct_Case 0 0 "NewEnumerator0"))
    (CallFunction|TestingWin)
    (Utilities|FlowControl|Delay 0.2)
    (Collision|SetCollisionProfileName (Variables|Default|GetBox_1) "BlockAllDynamic" true :!class /Script/Engine.PrimitiveComponent)))

(event OnComponentBeginOverlap(Box_2)
  (params (OverlappedComponent :type Primitive%20Component%20Object%20Reference) (OtherActor :type Actor%20Object%20Reference) (OtherComp :type Primitive%20Component%20Object%20Reference) (OtherBodyIndex :type Integer) (bFromSweep :type Boolean) (SweepResult :type Hit%20Result%20Structure%20%28by%20ref%29))
  (bind _box_2 (Variables|Default|GetBox_2))
  (bind _returnvalue (Transformation|GetRelativeTransform _box_2))
  (if (not (Variables|Default|GetBoxEnable2))
    (AddComponent|AddStaticMeshComponent false (Math|Transform|MakeTransform (.location _returnvalue) (.rotation _returnvalue) "1.000000,1.000000,1.000000"))
    (Variables|Default|SetBoxEnable2 true)
    (Utilities|Array|SetArrayElem (Variables|Default|GetGrilleArray) 1 (Utilities|Struct|MakeStruct_Case 1 0 "NewEnumerator0"))
    (CallFunction|TestingWin 1)
    (Utilities|FlowControl|Delay 0.2)
    (Collision|SetCollisionProfileName (Variables|Default|GetBox_2) "NoCollision" true :!class /Script/Engine.PrimitiveComponent)))

(event OnComponentBeginOverlap(Box_3)
  (params (OverlappedComponent :type Primitive%20Component%20Object%20Reference) (OtherActor :type Actor%20Object%20Reference) (OtherComp :type Primitive%20Component%20Object%20Reference) (OtherBodyIndex :type Integer) (bFromSweep :type Boolean) (SweepResult :type Hit%20Result%20Structure%20%28by%20ref%29))
  (bind _box_3 (Variables|Default|GetBox_3))
  (bind _returnvalue (Transformation|GetRelativeTransform _box_3))
  (if (not (Variables|Default|GetBoxEnable3))
    (AddComponent|AddStaticMeshComponent false (Math|Transform|MakeTransform (.location _returnvalue) (.rotation _returnvalue) "1.000000,1.000000,1.000000"))
    (Variables|Default|SetBoxEnable3 true)
    (Utilities|Array|SetArrayElem (Variables|Default|GetGrilleArray) 2 (Utilities|Struct|MakeStruct_Case 2 0 "NewEnumerator0"))
    (CallFunction|TestingWin 2)
    (Utilities|FlowControl|Delay 0.2)
    (Collision|SetCollisionProfileName (Variables|Default|GetBox_3) "NoCollision" true :!class /Script/Engine.PrimitiveComponent)))

(event OnComponentBeginOverlap(Box_4)
  (params (OverlappedComponent :type Primitive%20Component%20Object%20Reference) (OtherActor :type Actor%20Object%20Reference) (OtherComp :type Primitive%20Component%20Object%20Reference) (OtherBodyIndex :type Integer) (bFromSweep :type Boolean) (SweepResult :type Hit%20Result%20Structure%20%28by%20ref%29))
  (bind _box_4 (Variables|Default|GetBox_4))
  (bind _returnvalue (Transformation|GetRelativeTransform _box_4))
  (if (not (Variables|Default|GetBoxEnable4))
    (AddComponent|AddStaticMeshComponent false (Math|Transform|MakeTransform (.location _returnvalue) (.rotation _returnvalue) "1.000000,1.000000,1.000000"))
    (Variables|Default|SetBoxEnable4 true)
    (Utilities|Array|SetArrayElem (Variables|Default|GetGrilleArray) 3 (Utilities|Struct|MakeStruct_Case 0 1 "NewEnumerator0"))
    (CallFunction|TestingWin 3)
    (Utilities|FlowControl|Delay 0.2)
    (Collision|SetCollisionProfileName (Variables|Default|GetBox_4) "NoCollision" true :!class /Script/Engine.PrimitiveComponent)))

(event OnComponentBeginOverlap(Box_5)
  (params (OverlappedComponent :type Primitive%20Component%20Object%20Reference) (OtherActor :type Actor%20Object%20Reference) (OtherComp :type Primitive%20Component%20Object%20Reference) (OtherBodyIndex :type Integer) (bFromSweep :type Boolean) (SweepResult :type Hit%20Result%20Structure%20%28by%20ref%29))
  (bind _box_5 (Variables|Default|GetBox_5))
  (bind _returnvalue (Transformation|GetRelativeTransform _box_5))
  (if (not (Variables|Default|GetBoxEnable5))
    (AddComponent|AddStaticMeshComponent false (Math|Transform|MakeTransform (.location _returnvalue) (.rotation _returnvalue) "1.000000,1.000000,1.000000"))
    (Variables|Default|SetBoxEnable5 true)
    (Utilities|Array|SetArrayElem (Variables|Default|GetGrilleArray) 4 (Utilities|Struct|MakeStruct_Case 1 1 "NewEnumerator0"))
    (CallFunction|TestingWin 4)
    (Utilities|FlowControl|Delay 0.2)
    (Collision|SetCollisionProfileName (Variables|Default|GetBox_5) "NoCollision" true :!class /Script/Engine.PrimitiveComponent)))

(event OnComponentBeginOverlap(Box_6)
  (params (OverlappedComponent :type Primitive%20Component%20Object%20Reference) (OtherActor :type Actor%20Object%20Reference) (OtherComp :type Primitive%20Component%20Object%20Reference) (OtherBodyIndex :type Integer) (bFromSweep :type Boolean) (SweepResult :type Hit%20Result%20Structure%20%28by%20ref%29))
  (bind _box_6 (Variables|Default|GetBox_6))
  (bind _returnvalue (Transformation|GetRelativeTransform _box_6))
  (if (not (Variables|Default|GetBoxEnable6))
    (AddComponent|AddStaticMeshComponent false (Math|Transform|MakeTransform (.location _returnvalue) (.rotation _returnvalue) "1.000000,1.000000,1.000000"))
    (Variables|Default|SetBoxEnable6 true)
    (Utilities|Array|SetArrayElem (Variables|Default|GetGrilleArray) 5 (Utilities|Struct|MakeStruct_Case 2 1 "NewEnumerator0"))
    (CallFunction|TestingWin 5)
    (Utilities|FlowControl|Delay 0.2)
    (Collision|SetCollisionProfileName (Variables|Default|GetBox_6) "NoCollision" true :!class /Script/Engine.PrimitiveComponent)))

(event OnComponentBeginOverlap(Box_7)
  (params (OverlappedComponent :type Primitive%20Component%20Object%20Reference) (OtherActor :type Actor%20Object%20Reference) (OtherComp :type Primitive%20Component%20Object%20Reference) (OtherBodyIndex :type Integer) (bFromSweep :type Boolean) (SweepResult :type Hit%20Result%20Structure%20%28by%20ref%29))
  (bind _box_7 (Variables|Default|GetBox_7))
  (bind _returnvalue (Transformation|GetRelativeTransform _box_7))
  (if (not (Variables|Default|GetBoxEnable7))
    (AddComponent|AddStaticMeshComponent false (Math|Transform|MakeTransform (.location _returnvalue) (.rotation _returnvalue) "1.000000,1.000000,1.000000"))
    (Variables|Default|SetBoxEnable7 true)
    (Utilities|Array|SetArrayElem (Variables|Default|GetGrilleArray) 6 (Utilities|Struct|MakeStruct_Case 0 2 "NewEnumerator0"))
    (CallFunction|TestingWin 6)
    (Utilities|FlowControl|Delay 0.2)
    (Collision|SetCollisionProfileName (Variables|Default|GetBox_7) "NoCollision" true :!class /Script/Engine.PrimitiveComponent)))

(event OnComponentBeginOverlap(Box_8)
  (params (OverlappedComponent :type Primitive%20Component%20Object%20Reference) (OtherActor :type Actor%20Object%20Reference) (OtherComp :type Primitive%20Component%20Object%20Reference) (OtherBodyIndex :type Integer) (bFromSweep :type Boolean) (SweepResult :type Hit%20Result%20Structure%20%28by%20ref%29))
  (bind _box_8 (Variables|Default|GetBox_8))
  (bind _returnvalue (Transformation|GetRelativeTransform _box_8))
  (if (not (Variables|Default|GetBoxEnable8))
    (AddComponent|AddStaticMeshComponent false (Math|Transform|MakeTransform (.location _returnvalue) (.rotation _returnvalue) "1.000000,1.000000,1.000000"))
    (Variables|Default|SetBoxEnable7 true)
    (Utilities|Array|SetArrayElem (Variables|Default|GetGrilleArray) 7 (Utilities|Struct|MakeStruct_Case 1 2 "NewEnumerator0"))
    (CallFunction|TestingWin 7)
    (Utilities|FlowControl|Delay 0.2)
    (Collision|SetCollisionProfileName (Variables|Default|GetBox_8) "NoCollision" true :!class /Script/Engine.PrimitiveComponent)))

(event OnComponentBeginOverlap(Box_9)
  (params (OverlappedComponent :type Primitive%20Component%20Object%20Reference) (OtherActor :type Actor%20Object%20Reference) (OtherComp :type Primitive%20Component%20Object%20Reference) (OtherBodyIndex :type Integer) (bFromSweep :type Boolean) (SweepResult :type Hit%20Result%20Structure%20%28by%20ref%29))
  (bind _box_9 (Variables|Default|GetBox_9))
  (bind _returnvalue (Transformation|GetRelativeTransform _box_9))
  (if (not (Variables|Default|GetBoxEnable9))
    (AddComponent|AddStaticMeshComponent false (Math|Transform|MakeTransform (.location _returnvalue) (.rotation _returnvalue) "1.000000,1.000000,1.000000"))
    (Variables|Default|SetBoxEnable7 true)
    (Utilities|Array|SetArrayElem (Variables|Default|GetGrilleArray) 8 (Utilities|Struct|MakeStruct_Case 2 2 "NewEnumerator0"))
    (CallFunction|TestingWin 8)
    (Utilities|FlowControl|Delay 0.2)
    (Collision|SetCollisionProfileName (Variables|Default|GetBox_9) "NoCollision" true :!class /Script/Engine.PrimitiveComponent)))

(fn ConstructionScript)

(fn TestingWin
  (params (Index :type Integer))
  (Utilities|FlowControl|Sequence
    (:then_0
      (bind _iswin (CallFunction|TestingHorizontal Index))
      (if _iswin
        (Development|PrintString "Win")
        (return _iswin)))
    (:then_1
      (bind _iswin_2 (CallFunction|TestingVertical Index))
      (if _iswin_2
        (Development|PrintString "Win")
        (return _iswin_2)))
    (:then_2
      (bind _iswin_3 (CallFunction|TestingDiagonalGauche))
      (if _iswin_3
        (Development|PrintString "Win")
        (return _iswin_3)))
    (:then_3
      (bind _iswin_4 (CallFunction|TestingDiagonalDroite))
      (if _iswin_4
        (Development|PrintString "Win")
        (return _iswin_4)))))

(fn TestingHorizontal
  (params (Index :type Integer))
  (bind _grillearray (Variables|Default|GetGrilleArray))
  (bind _output (Utilities|Array|Get(acopy) _grillearray Index))
  (for _array_element (Variables|Default|GetGrilleArray)
    (if (== (.y _array_element) (.y _output))
      (if (== (Math|Conversions|ToInteger(Byte) (.value _array_element)) (Math|Conversions|ToInteger(Byte) (.value _output)))
        (Variables|Default|SetStreakPointValue (+ (Variables|Default|GetStreakPointValue) 1))
        (else
          (Variables|Default|SetStreakPointValue 0)))))
  (if (== (Variables|Default|GetStreakPointValue) 3)
    (return true)
    (else
      (Variables|Default|SetStreakPointValue 0)
      (return false))))

(fn TestingVertical
  (params (Index :type Integer))
  (bind _grillearray (Variables|Default|GetGrilleArray))
  (bind _output (Utilities|Array|Get(acopy) _grillearray))
  (for _array_element (Variables|Default|GetGrilleArray)
    (if (== (.x _array_element) (.x _output))
      (if (== (Math|Conversions|ToInteger(Byte) (.value _array_element)) (Math|Conversions|ToInteger(Byte) (.value _output)))
        (Variables|Default|SetStreakPointValue (+ (Variables|Default|GetStreakPointValue) 1))
        (else
          (Variables|Default|SetStreakPointValue 0)))))
  (if (== (Variables|Default|GetStreakPointValue) 3)
    (return true)
    (else
      (Variables|Default|SetStreakPointValue 0)
      (return false))))

(fn TestingDiagonalGauche
  (bind _grillearray (Variables|Default|GetGrilleArray))
  (bind _grillearray_2 (Variables|Default|GetGrilleArray))
  (bind _output (Utilities|Array|Get(acopy) _grillearray_2 4))
  (bind _output_2 (Utilities|Array|Get(acopy) _grillearray))
  (bind _returnvalue (Math|Conversions|ToInteger(Byte) (.value _output)))
  (bind _returnvalue_2 (Math|Conversions|ToInteger(Byte) (.value _output_2)))
  (if (!= _returnvalue_2 0)
    (if (== _returnvalue_2 _returnvalue)
      (if (== _returnvalue (Math|Conversions|ToInteger(Byte) (.value (Utilities|Array|Get(acopy) (Variables|Default|GetGrilleArray) 8))))
        (return true)
        (else
          _)))
    (return false)))

(fn TestingDiagonalDroite
  (bind _grillearray (Variables|Default|GetGrilleArray))
  (bind _grillearray_2 (Variables|Default|GetGrilleArray))
  (bind _output (Utilities|Array|Get(acopy) _grillearray_2 4))
  (bind _output_2 (Utilities|Array|Get(acopy) _grillearray 2))
  (bind _returnvalue (Math|Conversions|ToInteger(Byte) (.value _output)))
  (bind _returnvalue_2 (Math|Conversions|ToInteger(Byte) (.value _output_2)))
  (if (!= _returnvalue_2 0)
    (if (== _returnvalue_2 _returnvalue)
      (if (== _returnvalue (Math|Conversions|ToInteger(Byte) (.value (Utilities|Array|Get(acopy) (Variables|Default|GetGrilleArray) 6))))
        (return true)
        (else
          _)))
    (return false)))